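; Monster actor for a networked game that wanders and shows an overhead name tag, driven by its BP_MonsterEntity component.
; While the entity's ByControll flag is set, it loops AIMoveTo toward random points around the world origin, pausing briefly after success or failure.
; Outside dedicated servers, the widget yaws toward the camera each tick and displays name and entity ID once entity properties initialize.
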(event OnInitPropertiesFinishDelegate(BP_MonsterEntity)
  (if (not (Networking|IsDedicatedServer))
    (bind _ashead_ui (Utilities|Casting|CastToHeadUI (UserInterface|GetUserWidgetObject (Variables|Default|GetWidget))))
    (Rendering|Components|TextRender|SetText (Variables|/Game/UI/HeadUI.HeadUI_C|GetTextBlock_259 _ashead_ui) (Utilities|Text|FormatText "{0}[{1}]" (Utilities|Text|ToText(String) (Variables|/Script/MUEK.MonsterEntity|GetPlayerName (Variables|Default|GetBP_MonsterEntity))) (Variables|/Script/KBE.Entity|GetEntityID (Variables|Default|GetBP_MonsterEntity))))))

(event OnbyControllDelegate(BP_MonsterEntity)
  (params (IsByControll :type Boolean))
  (if IsByControll
    (CallFunction|FindLocationtoWalkto)))

(event Custom|Find%20Location%20to%20walk%20to
  (if (Variables|/Script/KBE.Entity|GetByControll (Variables|Default|GetBP_MonsterEntity))
    (AI|AIMoveTo self (* (Math|Random|RandomUnitVector) 1e+03) 0 25.0 false
      (:OnSuccess
        _)
      (:OnFail
        _))
    (Utilities|FlowControl|Delay (Math|Random|RandomFloatinRange 0.0 0.5))
    (CallFunction|FindLocationtoWalkto)))

(event EventBeginPlay)

(event Collision|EventActorBeginOverlap
  (params (OtherActor :type Actor%20Object%20Reference)))

(event EventTick
  (params (DeltaSeconds :type Float%20%28single-precision%29))
  (if (not (Networking|IsDedicatedServer))
    (Transformation|SetWorldRotation (Variables|Default|GetWidget) (Math|Rotator|MakeRotator 0.0 0.0 (.Yaw (Math|Rotator|BreakRotator (Math|Rotator|FindLookatRotation (Transformation|GetWorldLocation (Variables|Default|GetWidget)) (Camera|GetCameraLocation (Game|GetPlayerCameraManager 0)))))) false false)))

(fn ConstructionScript)