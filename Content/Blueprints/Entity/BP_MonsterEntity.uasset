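; BP_MonsterEntity is an entity Blueprint that passes follow and summon commands on to the monster that owns it.
; Its follow, stop-follow and come-here events each cast the owner to BP_Monster and call the matching function there, doing nothing if the cast fails.
; It holds no behavior of its own, as BeginPlay is empty and Tick is disabled.
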(event EventBeginPlay)

(event EventTick
  (params (DeltaSeconds :type Float%20%28single-precision%29)))

(event EventOnStopFollowMe
  (bind _asbp_monster (Utilities|Casting|CastToBP_Monster (Components|GetOwner)))
  (Class|KBEMonster|StopFollowMe _asbp_monster))

(event EventOnFollowMe
  (bind _asbp_monster (Utilities|Casting|CastToBP_Monster (Components|GetOwner)))
  (Class|KBEMonster|FollowMe _asbp_monster))

(event EventOnComeHere
  (bind _asbp_monster (Utilities|Casting|CastToBP_Monster (Components|GetOwner)))
  (Class|KBEMonster|ComeHere _asbp_monster))