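; BP_Follow is a pawn that follows its FollowActor using AI movement.
; A looping timer started on BeginPlay reissues AIMoveTo toward that actor several times a second while FollowMoveType equals 1.
; The OnGotoTarget event triggers the same move directly, skipping the type check.
; When a move succeeds or fails, the pawn snaps its rotation to that of its Owner, not the followed actor.
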(event Custom|CustomEvent_0
  (if (== (Variables|Default|GetFollowMoveType) 1)
    (AI|AIMoveTo self "0, 0, 0" (Variables|Default|GetFollowActor) 25.0 false
      (:OnSuccess
        _)
      (:OnFail
        _))
    (Transformation|SetActorRotation (Transformation|GetActorRotation (Components|GetOwner)))))

(event EventBeginPlay
  (Utilities|Time|SetTimerbyEvent (delegate Custom|CustomEvent_0) 0.1 true))

(event Collision|EventActorBeginOverlap
  (params (OtherActor :type Actor%20Object%20Reference)))

(event EventTick
  (params (DeltaSeconds :type Float%20%28single-precision%29)))

(event EventOnGotoTarget
  (AI|AIMoveTo self "0, 0, 0" (Variables|Default|GetFollowActor) 25.0 false
    (:OnSuccess
      _)
    (:OnFail
      _))
  (Transformation|SetActorRotation (Transformation|GetActorRotation (Components|GetOwner))))

(fn ConstructionScript)